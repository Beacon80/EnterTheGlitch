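; Gameplay game mode that creates two local players and manages which of three sibling characters each player controls.
; Siblings are stored in an array indexed by their enum value, and possession only succeeds on an unpossessed one.
; Next/previous switching wraps with modulo 3, using +2 to step backward, and skips one occupied sibling before printing that none are available.
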(event EventBeginPlay
  (bind _playerarray (Variables|Default|GetPlayerArray))
  (bind _returnvalue (Class|GameplayStatics|CreatePlayer 0))
  (Utilities|Array|Add _playerarray _returnvalue)
  (Class|GameplayStatics|CreatePlayer 1)
  (Utilities|Array|Add _playerarray 0))

(event Custom|PossessNextSibling
  (params (Player :type Integer) (CurrentSibling :type 0%20Sibling%20Object%20Reference) (isNext :type Boolean))
  (Variables|PossessNextSibling|SetPlayer Player)
  (if isNext
    (Variables|PossessNextSibling|SetModifier 1)
    (else
      (Variables|PossessNextSibling|SetModifier 2)))
  (if (Variables|/Game/Blueprints/Characters/Siblings/0_Sibling.0_Sibling_C|GetIsPossessed? (Utilities|Array|Get(acopy) (Variables|Siblings|GetSiblingArray) (Math|Integer|%(Integer) (+ (Math|Conversions|ToInteger(Byte) (Variables|/Game/Blueprints/Characters/Siblings/0_Sibling.0_Sibling_C|GetWhichSibling CurrentSibling)) (Variables|PossessNextSibling|GetModifier)) 3)))
    (if (Variables|/Game/Blueprints/Characters/Siblings/0_Sibling.0_Sibling_C|GetIsPossessed? (Utilities|Array|Get(acopy) (Variables|Siblings|GetSiblingArray) (Math|Integer|%(Integer) (+ (Math|Integer|%(Integer) (+ (Math|Conversions|ToInteger(Byte) (Variables|/Game/Blueprints/Characters/Siblings/0_Sibling.0_Sibling_C|GetWhichSibling CurrentSibling)) (Variables|PossessNextSibling|GetModifier)) 3) (Variables|PossessNextSibling|GetModifier)) 3)))
      (Development|PrintString "No Available Siblings")
      (else
        (CallFunction|PossessSibling (Variables|PossessNextSibling|GetPlayer) (Variables|/Game/Blueprints/Characters/Siblings/0_Sibling.0_Sibling_C|GetWhichSibling (Utilities|Array|Get(acopy) (Variables|Siblings|GetSiblingArray) (Math|Integer|%(Integer) (+ (Math|Integer|%(Integer) (+ (Math|Conversions|ToInteger(Byte) (Variables|/Game/Blueprints/Characters/Siblings/0_Sibling.0_Sibling_C|GetWhichSibling CurrentSibling)) (Variables|PossessNextSibling|GetModifier)) 3) (Variables|PossessNextSibling|GetModifier)) 3))))))
    (else
      (CallFunction|PossessSibling (Variables|PossessNextSibling|GetPlayer) (Variables|/Game/Blueprints/Characters/Siblings/0_Sibling.0_Sibling_C|GetWhichSibling (Utilities|Array|Get(acopy) (Variables|Siblings|GetSiblingArray) (Math|Integer|%(Integer) (+ (Math|Conversions|ToInteger(Byte) (Variables|/Game/Blueprints/Characters/Siblings/0_Sibling.0_Sibling_C|GetWhichSibling CurrentSibling)) (Variables|PossessNextSibling|GetModifier)) 3)))))))

(event Custom|AddSiblingActor
  (params (Sibling :type 0%20Sibling%20Object%20Reference))
  ;[1 1 1] Adds/Updates a sibling to the array
  (Utilities|Array|SetArrayElem (Variables|Siblings|GetSiblingArray) (Math|Conversions|ToInteger(Byte) (Variables|/Game/Blueprints/Characters/Siblings/0_Sibling.0_Sibling_C|GetWhichSibling Sibling)) Sibling))

(event Custom|PossessSibling
  (params (Player :type Integer) (Sibling :type En_Sibling%20Enum :default "NewEnumerator0"))
  (bind _returnvalue (Math|Conversions|ToInteger(Byte) Sibling))
  (bind _siblingarray (Variables|Siblings|GetSiblingArray))
  (bind _output (Utilities|Array|Get(acopy) _siblingarray _returnvalue))
  ;[1 1 1] Possess a specific sibling
  (if (not (Variables|/Game/Blueprints/Characters/Siblings/0_Sibling.0_Sibling_C|GetIsPossessed? _output))
    (Pawn|Possess (Game|GetPlayerController Player) _output)))

(fn ConstructionScript)