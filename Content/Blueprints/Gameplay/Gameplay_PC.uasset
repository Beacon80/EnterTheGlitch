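; Gameplay player controller that handles input for switching which sibling character each player controls.
; It caches the Gameplay_GM game mode on BeginPlay and forwards released input actions to its possession functions.
; Player one can pick Jenn, Ner or Rick directly or cycle to the next or previous sibling.
; The same controller also cycles player two to the next sibling, using the pawn of player controller index 1.
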(event EventBeginPlay
  (Variables|Default|SetGameplay_GM (.AsGameplay%20GM (Utilities|Casting|CastToGameplay_GM (Game|GetGameMode)))))

(event Input|ActionEvents|InputActionPossessRick1P
  (params (Key :type Key%20Structure :default "None"))
  (:Released
    (Default|PossessSibling (Variables|Default|GetGameplay_GM) 0 "NewEnumerator2")))

(event Input|ActionEvents|InputActionPossessNext
  (params (Key :type Key%20Structure :default "None"))
  (:Released
    (Default|PossessNextSibling (Variables|Default|GetGameplay_GM) 0 (.As0%20Sibling (Utilities|Casting|CastTo0_Sibling (Pawn|GetControlledPawn))) true)))

(event Input|ActionEvents|InputActionPossessPrev
  (params (Key :type Key%20Structure :default "None"))
  (:Released
    (Default|PossessNextSibling (Variables|Default|GetGameplay_GM) 0 (.As0%20Sibling (Utilities|Casting|CastTo0_Sibling (Pawn|GetControlledPawn))) false)))

(event Input|ActionEvents|InputActionPossess2P
  (params (Key :type Key%20Structure :default "None"))
  (:Released
    (Default|PossessNextSibling (Variables|Default|GetGameplay_GM) 1 (.As0%20Sibling (Utilities|Casting|CastTo0_Sibling (Pawn|GetControlledPawn (Game|GetPlayerController 1)))) true)))

(event Input|ActionEvents|InputActionPossessJenn1P
  (params (Key :type Key%20Structure :default "None"))
  (:Released
    (Default|PossessSibling (Variables|Default|GetGameplay_GM) 0 "NewEnumerator0")))

(event Input|ActionEvents|InputActionPossessNer1P
  (params (Key :type Key%20Structure :default "None"))
  (:Released
    (Default|PossessSibling (Variables|Default|GetGameplay_GM) 0 "NewEnumerator1")))

(fn ConstructionScript)